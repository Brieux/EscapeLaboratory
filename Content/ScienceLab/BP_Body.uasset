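; BP_Body is the player-controlled body in the ScienceLab, handling movement and view rotation.
; On possession it adds the IMC_Movement Enhanced Input context, with IA_Move driving movement along actor axes and IA_Turn driving yaw and pitch; legacy axis events remain empty.
; Overlapping actors receive a CheckIDMessage call carrying a hard-coded ID.
; The construction script calls AddAC0X00A21E, whose purpose is not shown.
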(event `self.ReceivePossessed`
  (params (NewController :type "Controller Object Reference"))
  ;[1 0 0] Initializing Neural connections
  (bind _asplayer_controller (cast `PlayerController` NewController))
  (`EnhancedInputSubsystemInterface.AddMappingContext` (pcsubsystem `EnhancedInputLocalPlayerSubsystem` _asplayer_controller) "/Game/ScienceLab/IMC_Movement.IMC_Movement" 0))

(event `InputAxis|MoveForward` :consume false :overrideparent false
  (params (AxisValue :type "Float (single-precision)"))
  ;[0 0.3281 0] OLD
)

(event `EnhancedInput|/Game/ScienceLab/IA_Move`
  (params (ActionValue :type "Vector2D Structure") (ElapsedSeconds :type "Float (single-precision)") (TriggeredSeconds :type "Float (single-precision)"))
  ;[0.006671 0.151 0] Controls
  (:`Triggered`
    (`self.AddMovementInput` (+ (* ActionValue_X (`self.GetActorForwardVector`)) (* ActionValue_Y (`self.GetActorRightVector`))))))

(event `InputAxis|MoveRight` :consume false :overrideparent false
  (params (AxisValue :type "Float (single-precision)"))
  ;[0 0.3281 0] OLD
)

(event `InputAxis|Turn` :overrideparent false
  (params (AxisValue :type "Float (single-precision)"))
  ;[0 0.3281 0] OLD
)

(event `EnhancedInput|/Game/ScienceLab/IA_Turn`
  (params (ActionValue :type "Vector2D Structure") (ElapsedSeconds :type "Float (single-precision)") (TriggeredSeconds :type "Float (single-precision)"))
  ;[0.006671 0.151 0] HeadRotation
  (:`Triggered`
    (`self.AddControllerYawInput` ActionValue_X)
    (`self.AddControllerPitchInput` ActionValue_Y)))

(event `InputAxis|LookUp` :overrideparent false
  (params (AxisValue :type "Float (single-precision)"))
  ;[0 0.3281 0] OLD
)

(event `self.ReceiveActorBeginOverlap`
  (params (OtherActor :type "Actor Object Reference"))
  ;[1 0 0] ID
  (message `/Game/ScienceLab/SecuritySystem/BPI_Identity.CheckID` OtherActor "id_29"))

(fn `UserConstructionScript`
  (`|ExecutionSequence`
    (:`then_0`
      (`AddComponent|NODE_AddAC_0X00A21E-0`))
    (:`then_1`)))